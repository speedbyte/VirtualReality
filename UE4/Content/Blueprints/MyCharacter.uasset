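; MyCharacter is a player character with axis-driven movement, strafing and camera look, plus an F-key interaction for activating quadcopters.
; Movement follows the control rotation's forward and right vectors, while the look axes feed controller pitch and yaw.
; Pressing F runs a short Visibility line trace from the camera and calls ActivateQuadcopterMessage on the hit actor.
; A SpawnActor node near the "Shoot Fireballs" comment is disconnected and never runs.
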(event Input|AxisEvents|InputAxisMoveForward
  (params (AxisValue :type Float%20%28single-precision%29))
  ;[1 1 1] Movements
  (Pawn|Input|AddMovementInput (Math|Vector|GetForwardVector (Pawn|GetControlRotation :!class /Script/Engine.Pawn)) AxisValue false))

(event Input|AxisEvents|InputAxisLookUp
  (params (AxisValue :type Float%20%28single-precision%29))
  ;[1 1 1] Directions
  (Pawn|Input|AddControllerPitchInput AxisValue))

(event Input|AxisEvents|InputAxisStrafeLeft
  (params (AxisValue :type Float%20%28single-precision%29))
  ;[1 1 1] Movements
  (Pawn|Input|AddMovementInput (Math|Vector|GetRightVector (Pawn|GetControlRotation :!class /Script/Engine.Pawn)) AxisValue false))

(event Input|AxisEvents|InputAxisLookLeft
  (params (AxisValue :type Float%20%28single-precision%29))
  ;[1 1 1] Directions
  (Pawn|Input|AddControllerYawInput AxisValue))

(event Input|KeyboardEvents|F
  (params (Key :type Key%20Structure :default "AnyKey"))
  (bind _camera (Variables|Default|GetCamera))
  (bind _returnvalue (Transformation|GetWorldLocation _camera))
  ;[1 1 1] F key pressed send event
  (:Pressed
    (bind (_outhit _returnvalue_2) (Collision|LineTraceByChannel _returnvalue (+ _returnvalue (* (Math|Vector|GetForwardVector (Transformation|GetWorldRotation _camera)) 3e+02)) "TraceTypeQuery1" false 0 "None"))
    (if _returnvalue_2
      (Class|InteractionInterface|ActivateQuadcopter(Message) (.HitActor (Collision|BreakHitResult _outhit))))))

(event Input|MouseEvents|LeftMouseButton
  (params (Key :type Key%20Structure :default "AnyKey"))
  ;[1 1 1] Shoot Fireballs
)

(event Input|KeyboardEvents|F
  (params (Key :type Key%20Structure :default "AnyKey")))

(fn ConstructionScript)