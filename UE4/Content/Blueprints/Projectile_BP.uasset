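; Projectile actor with four spinning propellers, apparently a quadcopter-style drone.
; Tick advances a wrapping yaw angle for the propellers and periodically prepends a location to a printed debug string, clearing it roughly every five seconds.
; A separate event sweeps the Box to a supplied location.
; When projectile movement stops, rotating movement halts and physics simulation takes over; velocity and random-rotation logic is left unconnected.
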(event OnProjectileStop(ProjectileMovement)
  (params (ImpactResult :type Hit%20Result%20Structure%20%28by%20ref%29))
  ;[1 1 1] Stop behaviors of the projectile
  (Variables|/Script/Engine.RotatingMovementComponent|SetRotationRate (Variables|Default|GetRotatingMovement) "0, 0, 0")
  (Physics|SetSimulatePhysics (Variables|/Script/Engine.MovementComponent|GetUpdatedPrimitive (Variables|Default|GetProjectileMovement)) true))

(event Collision|EventActorBeginOverlap
  (params (OtherActor :type Actor%20Object%20Reference)))

(event EventTick
  (params (DeltaSeconds :type Float%20%28single-precision%29))
  ;[1 1 1] Animation of the Propeller
  (bind _output_get (Variables|Default|SetRotationInAngle (+ (* DeltaSeconds (Variables|Default|GetRotationRate)) (Variables|Default|GetRotationInAngle))))
  (if (< _output_get 361.0)
    _
    (else
      (bind _output_get_2 (Variables|Default|SetRotationInAngle 0.0))))
  (Transformation|SetRelativeRotation (Variables|Default|GetPropeller4) (Math|Rotator|MakeRotator 0.0 0.0 _output_get_2) false false)
  (Transformation|SetRelativeRotation (Variables|Default|GetPropeller1) (Math|Rotator|MakeRotator 0.0 0.0 _output_get_2) false false)
  (Transformation|SetRelativeRotation (Variables|Default|GetPropeller2) (Math|Rotator|MakeRotator 0.0 0.0 _output_get_2) false false)
  (Transformation|SetRelativeRotation (Variables|Default|GetPropeller3) (Math|Rotator|MakeRotator 0.0 0.0 _output_get_2) false false)
  ;[1 1 1] Moving Behavior every tick
  (bind _output_get_3 (Variables|Default|SetcounterVal_Step (+ DeltaSeconds (Variables|Default|GetcounterVal_Step))))
  (if (>= _output_get_3 0.3)
    (Variables|Default|SetcounterVal_Step 0.0)
    (bind _output_get_4 (Variables|Default|SetstringVal (Utilities|String|Append (Utilities|String|ToString(Vector) (stale Event?wtf location)) (Variables|Default|GetstringVal))))
    (Development|PrintString _output_get_4)
    (bind _output_get_5 (Variables|Default|SetcounterVal_Send (+ 0.3 (Variables|Default|GetcounterVal_Send))))
    (if (>= _output_get_5 5.0)
      (Variables|Default|SetcounterVal_Send 0.0)
      (Variables|Default|SetstringVal "")
      (Development|PrintString ""))))

(event Event?wtf
  (params (location :type Vector))
  ;[1 1 1] Moving Behavior every tick
  (Transformation|SetWorldLocation (Variables|Default|GetBox) location true false))

(fn ConstructionScript)